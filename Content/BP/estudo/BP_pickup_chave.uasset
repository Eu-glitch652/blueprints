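; Key pickup that unlocks a linked door by granting it the key when the player interacts.
; Sphere overlap registers the pickup as the BP_ThirdPersonCharacter's last interactable and enables interaction, which end overlap disables.
; When allowed, the Interagir event calls Corpo, sets TemChave on the referenced Porta and destroys the pickup.
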(event OnComponentBeginOverlap(Sphere)
  (params (OverlappedComponent :type Primitive%20Component%20Object%20Reference) (OtherActor :type Actor%20Object%20Reference) (OtherComp :type Primitive%20Component%20Object%20Reference) (OtherBodyIndex :type Integer) (bFromSweep :type Boolean) (SweepResult :type Hit%20Result%20Structure%20%28by%20ref%29))
  (bind _asbp_third_person_character (Utilities|Casting|CastToBP_ThirdPersonCharacter OtherActor))
  (Variables|/Game/ThirdPerson/Blueprints/BP_ThirdPersonCharacter.BP_ThirdPersonCharacter_C|SetUltimoInteragivel _asbp_third_person_character self)
  (Variables|Default|SetPodeinteragir? true))

(event OnComponentEndOverlap(Sphere)
  (params (OverlappedComponent :type Primitive%20Component%20Object%20Reference) (OtherActor :type Actor%20Object%20Reference) (OtherComp :type Primitive%20Component%20Object%20Reference) (OtherBodyIndex :type Integer))
  (Utilities|Casting|CastToBP_ThirdPersonCharacter OtherActor)
  (Variables|Default|SetPodeinteragir? false))

(event EventInteragir
  (if (Variables|Default|GetPodeinteragir?)
    (CallFunction|Corpo)
    (Variables|/Game/BP/estudo/BP_door.BP_door_C|SetTemChave? (Variables|Default|GetPorta) true)
    (Actor|DestroyActor)))

(fn ConstructionScript
  (|CallParentFunction))