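; Master pickup actor that the third-person character can interact with while inside its sphere.
; Sphere overlap registers it as the character's UltimoInteragivel and enables interaction; leaving disables interaction but keeps that reference.
; When allowed, Interagir calls the empty Corpo event, apparently a hook for child pickups, then destroys the actor and prints a debug message.
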(event OnComponentBeginOverlap(Sphere)
  (params (OverlappedComponent :type Primitive%20Component%20Object%20Reference) (OtherActor :type Actor%20Object%20Reference) (OtherComp :type Primitive%20Component%20Object%20Reference) (OtherBodyIndex :type Integer) (bFromSweep :type Boolean) (SweepResult :type Hit%20Result%20Structure%20%28by%20ref%29))
  (bind _asbp_third_person_character (Utilities|Casting|CastToBP_ThirdPersonCharacter OtherActor))
  (Variables|/Game/ThirdPerson/Blueprints/BP_ThirdPersonCharacter.BP_ThirdPersonCharacter_C|SetUltimoInteragivel _asbp_third_person_character self)
  (Variables|Default|SetpodeInteragir true))

(event OnComponentEndOverlap(Sphere)
  (params (OverlappedComponent :type Primitive%20Component%20Object%20Reference) (OtherActor :type Actor%20Object%20Reference) (OtherComp :type Primitive%20Component%20Object%20Reference) (OtherBodyIndex :type Integer))
  (Utilities|Casting|CastToBP_ThirdPersonCharacter OtherActor)
  (Variables|Default|SetpodeInteragir false))

(event Custom|corpo)

(event EventInteragir
  (if (Variables|Default|GetpodeInteragir)
    (CallFunction|Corpo)
    (Actor|DestroyActor)
    (Development|PrintString "destruiu")))

(fn ConstructionScript)