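; BP_porta is a door that swings open when something overlaps its box, provided its TemChave (has key) flag is set.
; The LinhaDoTempo timeline drives the static mesh's relative yaw and, on finishing, sets PortaAberta from whether the final value is above zero.
; Ending the overlap reverses the timeline only if PortaAberta is already true, so leaving mid-swing does not close the door.
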(event OnComponentBeginOverlap(Box)
  (params (OverlappedComponent :type Primitive%20Component%20Object%20Reference) (OtherActor :type Actor%20Object%20Reference) (OtherComp :type Primitive%20Component%20Object%20Reference) (OtherBodyIndex :type Integer) (bFromSweep :type Boolean) (SweepResult :type Hit%20Result%20Structure%20%28by%20ref%29))
  (if (Variables|Default|GetTemChave?)
    (if (not (Variables|Default|GetportaAberta?))
      (bind _nova_faixa_0 (Timeline|Linha%20do%20tempo PlayFromStart)
        (:Update
          (Transformation|SetRelativeRotation (Variables|Default|GetStaticMesh) (Math|Rotator|MakeRotator 0.0 0.0 _nova_faixa_0) false false))
        (:Finished
          (Variables|Default|SetportaAberta? (> _nova_faixa_0 0.0)))))))

(event OnComponentEndOverlap(Box)
  (params (OverlappedComponent :type Primitive%20Component%20Object%20Reference) (OtherActor :type Actor%20Object%20Reference) (OtherComp :type Primitive%20Component%20Object%20Reference) (OtherBodyIndex :type Integer))
  (if (Variables|Default|GetportaAberta?)
    (bind _nova_faixa_0 (Timeline|Linha%20do%20tempo ReverseFromEnd)
      (:Update
        (Transformation|SetRelativeRotation (Variables|Default|GetStaticMesh) (Math|Rotator|MakeRotator 0.0 0.0 _nova_faixa_0) false false))
      (:Finished
        (Variables|Default|SetportaAberta? (> _nova_faixa_0 0.0))))))

(fn ConstructionScript)